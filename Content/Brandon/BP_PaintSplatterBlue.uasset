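; Blue paint splatter actor that plays an impact sound and leaves a temporary paint decal where it hits.
; On hit, a DoOnce plays SCImpact, waits half a second, then resets and spawns a short-lived M_PaintSplat decal aligned to the surface normal.
; A dynamic material instance picks a random splat frame; the SplatColour parameter setter is unconnected, and MakeSound is empty.
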(event `self.ReceiveHit`
  (params (MyComp :type "PrimitiveComponent Object Reference") (Other :type "Actor Object Reference") (OtherComp :type "PrimitiveComponent Object Reference") (bSelfMoved :type Boolean) (HitLocation :type "Vector Structure") (HitNormal :type "Vector Structure") (NormalImpulse :type "Vector Structure") (Hit :type "HitResult Structure (by ref)"))
  (`/Engine/EditorBlueprintResources/StandardMacros.DoOnce` false :!label _label
    (:`Completed`
      (`AudioComponent.Play` (`self.SC_Impact`) 0.0)
      (`KismetSystemLibrary.Delay` 0.5)
      (`|ExecutionSequence`
        (:`then_0`
          (goto _label :!via `Reset`))
        (:`then_1`
          (bind _returnvalue (`GameplayStatics.SpawnDecalAtLocation` "/Game/Brandon/M_PaintSplat.M_PaintSplat" (40.0 40.0 0.0) HitLocation (`KismetMathLibrary.Conv_VectorToRotator` HitNormal) 5.0))
          (bind _returnvalue_2 (`DecalComponent.CreateDynamicMaterialInstance` _returnvalue))
          (`MaterialInstanceDynamic.SetScalarParameterValue` _returnvalue_2 "Frame" (`KismetMathLibrary.Conv_IntToDouble` (`KismetMathLibrary.RandomIntegerInRange` 0 3))))))))

(fn `MakeSound`)

(fn `UserConstructionScript`)