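; BP_Disc is a menu disc actor that animates a disk insertion and then switches on the PC menu screen.
; InsertDisk reveals the mesh, waits briefly, then a timeline lerps it along its local Y axis.
; When the timeline finishes, it calls TurnOnScreen on every BP_PCMenu found in the level, with a delayed self-destroy chained from the loop body.
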(event `InsertDisk`
  (`SceneComponent.SetVisibility` (`self.StaticMesh`) true false)
  (`KismetSystemLibrary.Delay` 2.0)
  (bind (_direction _move) (`Timeline|Timeline`)
    (:`Update`
      (`SceneComponent.K2_SetRelativeLocation` (`self.StaticMesh`) (`KismetMathLibrary.MakeVector` 0.0 (`KismetMathLibrary.Lerp` 0.0 -40.0 _move)) false false))
    (:`Finished`
      (bind _outactors (`GameplayStatics.GetAllActorsOfClass` "/Game/Blueprints/Menu/BP_PCMenu.BP_PCMenu_C"))
      (for _array_element _outactors
        (`/Game/Blueprints/Menu/BP_PCMenu.TurnOnScreen` _array_element)
        (`KismetSystemLibrary.Delay` 0.2)
        (`self.K2_DestroyActor`)))))

(fn `UserConstructionScript`)