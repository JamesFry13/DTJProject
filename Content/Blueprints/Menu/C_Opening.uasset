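; Opening-sequence Blueprint that takes the player from an intro fade-in to the Brandon level through an in-world PC.
; BeginPlay fades the camera in, then shows a WBP_MenuPrompt after a delay.
; Pressing E removes the prompt, calls InsertDisk on BP_Disc actors and starts a timer for ZoomIntoScreen.
; That function sets camera FOV, blends the view to BP_PCMenu, fades out and opens the level via another timer.
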(event `self.ReceiveBeginPlay`
  (bind _returnvalue (`GameplayStatics.GetPlayerController` 0))
  (`self.CameraFade`)
  (`WidgetBlueprintLibrary.SetInputMode_GameAndUIEx` _returnvalue null)
  (set `PlayerController.bEnableClickEvents` true _returnvalue)
  (`KismetSystemLibrary.Delay` 4.0)
  (bind _returnvalue_2 (`|CreateWidget` "/Game/Blueprints/Menu/WBP_MenuPrompt.WBP_MenuPrompt_C"))
  (bind _returnvalue_3 (`UserWidget.AddToPlayerScreen` _returnvalue_2 0)))

(event `Key|E`
  (params (Key :type "Key Structure"))
  (:`Pressed`
    (if (stale `self.ReceiveBeginPlay` _returnvalue_3)
      (`Widget.RemoveFromParent` (stale `self.ReceiveBeginPlay` _returnvalue_2))
      (bind _outactors (`GameplayStatics.GetAllActorsOfClass` "/Game/Blueprints/Menu/BP_Disc.BP_Disc_C"))
      (for _array_element _outactors
        (`/Game/Blueprints/Menu/BP_Disc.InsertDisk` _array_element)
        (`WidgetBlueprintLibrary.SetInputMode_UIOnlyEx` (`GameplayStatics.GetPlayerController` 0) null)
        (`KismetSystemLibrary.K2_SetTimer` null "ZoomIntoScreen" 3.0)))))

(fn `CameraFade`
  (`PlayerCameraManager.StartCameraFade` :`self` (`GameplayStatics.GetPlayerCameraManager` 0) :`FromAlpha` 1.5 :`Duration` 2.0 :`bShouldFadeAudio` true))

(fn `Open`
  (`GameplayStatics.OpenLevelBySoftObjectPtr` "/Game/Levels/Brandon.Brandon"))

(fn `UserConstructionScript`)

(fn `ZoomIntoScreen`
  (bind _returnvalue (`GameplayStatics.GetPlayerController` 0))
  (`CameraComponent.SetFieldOfView` (`self.Camera`) 60.0)
  (bind _outactors (`GameplayStatics.GetAllActorsOfClass` "/Game/Blueprints/Menu/BP_PCMenu.BP_PCMenu_C"))
  (for _array_element _outactors
    (`PlayerController.SetViewTargetWithBlend` _returnvalue _array_element 1.5 "VTBlend_Linear" 1.0 false)
    (`WidgetBlueprintLibrary.SetInputMode_UIOnlyEx` _returnvalue null)
    (set `PlayerController.bShowMouseCursor` true _returnvalue)
    (`PlayerCameraManager.StartCameraFade` :`self` (`GameplayStatics.GetPlayerCameraManager` 0) :`ToAlpha` 2.0 :`Duration` 2.0 :`bHoldWhenFinished` true)
    (`KismetSystemLibrary.K2_SetTimer` null "Open" 2.0)))