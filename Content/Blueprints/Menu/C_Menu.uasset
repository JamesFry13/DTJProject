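; C_Menu is the main menu Blueprint that fades the camera in and stages the transition from the menu into the Brandon level.
; On BeginPlay it starts the fade with audio and enables click events with Game and UI input.
; ZoomIntoScreen, not called within this Blueprint, sets the camera FOV, blends the view to BP_PCMenu, switches to UI-only input and fades out.
; A timer then calls Open by name to load the level.
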(event `self.ReceiveBeginPlay`
  (bind _returnvalue (`GameplayStatics.GetPlayerController` 0))
  (`self.CameraFade`)
  (`WidgetBlueprintLibrary.SetInputMode_GameAndUIEx` _returnvalue null)
  (set `PlayerController.bEnableClickEvents` true _returnvalue)
  (`KismetSystemLibrary.Delay` 4.0))

(fn `CameraFade`
  (`PlayerCameraManager.StartCameraFade` :`self` (`GameplayStatics.GetPlayerCameraManager` 0) :`FromAlpha` 1.5 :`Duration` 2.0 :`bShouldFadeAudio` true))

(fn `Open`
  (`GameplayStatics.OpenLevelBySoftObjectPtr` "/Game/Levels/Brandon.Brandon"))

(fn `UserConstructionScript`)

(fn `ZoomIntoScreen`
  (bind _returnvalue (`GameplayStatics.GetPlayerController` 0))
  (`CameraComponent.SetFieldOfView` (`self.Camera`) 60.0)
  (bind _outactors (`GameplayStatics.GetAllActorsOfClass` "/Game/Blueprints/Menu/BP_PCMenu.BP_PCMenu_C"))
  (for _array_element _outactors
    (`PlayerController.SetViewTargetWithBlend` _returnvalue _array_element 1.5 "VTBlend_Linear" 1.0 false)
    (`WidgetBlueprintLibrary.SetInputMode_UIOnlyEx` _returnvalue null)
    (set `PlayerController.bShowMouseCursor` true _returnvalue)
    (`PlayerCameraManager.StartCameraFade` :`self` (`GameplayStatics.GetPlayerCameraManager` 0) :`ToAlpha` 2.0 :`Duration` 2.0)
    (`KismetSystemLibrary.K2_SetTimer` null "Open" 2.0)))