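; BP_DoorBase is a door Blueprint that slides its Cube mesh vertically when opened.
; DoorOpen passes through a DoOnce, prints a debug string, then plays a timeline that lerps the mesh's relative Z upward.
; The construction script applies the DoorMesh and DoorScale variables to the Cube.
; DoorClose is an empty event and nothing resets the DoOnce, so the door opens only once.
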(event `self.ReceiveBeginPlay`)

(event `DoorOpen`
  (`/Engine/EditorBlueprintResources/StandardMacros.DoOnce` false
    (:`Completed`
      (`KismetSystemLibrary.PrintString` "Hello")
      (bind (_direction _move) (`Timeline|Timeline`)
        (:`Update`
          (`SceneComponent.K2_SetRelativeLocation` (`self.Cube`) (`KismetMathLibrary.MakeVector` 0.0 0.0 (`KismetMathLibrary.Lerp` 320.0 600.0 _move)) false false))))))

(event `DoorClose`)

(fn `UserConstructionScript`
  (locals (NewLocalVar :type "StaticMeshComponent Object Reference"))
  (bind _cube (`self.Cube`))
  (set `self.DoorValue` (`self.DoorValue`))
  (`SceneComponent.SetWorldScale3D` _cube (`self.DoorScale`))
  (`StaticMeshComponent.SetStaticMesh` _cube (`self.DoorMesh`)))