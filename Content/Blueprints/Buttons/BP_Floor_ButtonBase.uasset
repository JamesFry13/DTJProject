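; Base floor button that is pressed when a component tagged Pickup overlaps its collider, with an empty ButtonAction event as the hook for what it triggers.
; A press briefly enables physics on the button mesh, then disables it, sets a plane constraint and calls ButtonAction.
; Any end overlap, regardless of tag, returns the button to its saved start location and re-arms the DoOnce after a short delay.
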(event `self.ReceiveBeginPlay`
  ; Save origin location
  (set `self.OriginLoc` (`SceneComponent.K2_GetComponentLocation` (`self.Button`))))

(event `self.OverlapCollider.OnComponentBeginOverlap`
  (params (OverlappedComponent :type "PrimitiveComponent Object Reference") (OtherActor :type "Actor Object Reference") (OtherComp :type "PrimitiveComponent Object Reference") (OtherBodyIndex :type Integer) (bFromSweep :type Boolean) (SweepResult :type "HitResult Structure (by ref)"))
  (bind _button (`self.Button`))
  ; Press
  (if (`ActorComponent.ComponentHasTag` OtherComp "Pickup")
    (`/Engine/EditorBlueprintResources/StandardMacros.DoOnce` false :!label _label
      (:`Completed`
        (set `self.IsPressed?` true)
        (`PrimitiveComponent.SetSimulatePhysics` _button true)
        (`KismetSystemLibrary.Delay` 0.5)
        (`PrimitiveComponent.SetSimulatePhysics` _button false)
        (`PrimitiveComponent.SetConstraintMode` _button "XYPlane")
        (`self.ButtonAction`)))))

(event `self.OverlapCollider.OnComponentEndOverlap`
  (params (OverlappedComponent :type "PrimitiveComponent Object Reference") (OtherActor :type "Actor Object Reference") (OtherComp :type "PrimitiveComponent Object Reference") (OtherBodyIndex :type Integer))
  ; Depress
  (`SceneComponent.K2_SetWorldLocation` (`self.Button`) (`self.OriginLoc`) false false)
  (set `self.IsPressed?` false)
  (`KismetSystemLibrary.Delay` 0.2)
  (goto _label :!via `Reset`))

(event `ButtonAction`)

(fn `UserConstructionScript`)