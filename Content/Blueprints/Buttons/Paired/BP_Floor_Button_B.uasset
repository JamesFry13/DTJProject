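; Floor button B of a two-button pair that opens matching two-button doors.
; A Pickup-tagged component overlap triggers a DoOnce press, briefly simulating physics on the button before checking for any pressed BP_Floor_Button_A and opening doors sharing its ButtonValue.
; Any end overlap restores the button's position, resets the DoOnce and, after a short delay, closes two-button doors regardless of value.
; Both transitions play a click sound.
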(event `self.ReceiveBeginPlay`
  ; Save origin location
  (set `self.OriginLoc` (`SceneComponent.K2_GetComponentLocation` (`self.Button`))))

(event `self.OverlapCollider.OnComponentBeginOverlap`
  (params (OverlappedComponent :type "PrimitiveComponent Object Reference") (OtherActor :type "Actor Object Reference") (OtherComp :type "PrimitiveComponent Object Reference") (OtherBodyIndex :type Integer) (bFromSweep :type Boolean) (SweepResult :type "HitResult Structure (by ref)"))
  (bind _button (`self.Button`))
  ; Press
  (if (`ActorComponent.ComponentHasTag` OtherComp "Pickup")
    (`/Engine/EditorBlueprintResources/StandardMacros.DoOnce` false :!label _label
      (:`Completed`
        (set `self.IsPressed?` true)
        (`PrimitiveComponent.SetSimulatePhysics` _button true)
        (`KismetSystemLibrary.Delay` 0.5)
        (`PrimitiveComponent.SetSimulatePhysics` _button false)
        (`PrimitiveComponent.SetConstraintMode` _button "XYPlane")
        (`self.ButtonBPressed`)
        (set `self.ButtonBPressed?` true)))))

(event `self.OverlapCollider.OnComponentEndOverlap`
  (params (OverlappedComponent :type "PrimitiveComponent Object Reference") (OtherActor :type "Actor Object Reference") (OtherComp :type "PrimitiveComponent Object Reference") (OtherBodyIndex :type Integer))
  ; Depress
  (`SceneComponent.K2_SetWorldLocation` (`self.Button`) (`self.OriginLoc`) false false)
  (set `self.IsPressed?` false)
  (`KismetSystemLibrary.Delay` 0.2)
  (`self.ButtonDepressed`)
  (set `self.ButtonBPressed?` false)
  (goto _label :!via `Reset`))

(event `ButtonBPressed`
  ; Finds corresponding door by value
  (`self.PlaySound`)
  (bind _outactors (`GameplayStatics.GetAllActorsOfClass` "/Game/Blueprints/Buttons/Paired/BP_Floor_Button_A.BP_Floor_Button_A_C"))
  (for _array_element _outactors
    (if (`/Game/Blueprints/Buttons/Paired/BP_Floor_Button_A.ButtonAPressed?` _array_element)
      (bind _outactors_2 (`GameplayStatics.GetAllActorsOfClass` "/Game/Blueprints/BP_DoorBase.BP_DoorBase_C"))
      (for _array_element_2 _outactors_2
        (bind _asbp_door_2button (cast `/Game/Blueprints/BP_Door_2Button` _array_element_2))
        (if (== (`self.ButtonValue`) (`/Game/Blueprints/BP_Door_2Button.2DoorValue` _asbp_door_2button))
          (`/Game/Blueprints/BP_DoorBase.DoorOpen` _asbp_door_2button))))))

(event `ButtonDepressed`
  ; Comment
  (`self.PlaySound`)
  (bind _outactors (`GameplayStatics.GetAllActorsOfClass` "/Game/Blueprints/BP_DoorBase.BP_DoorBase_C"))
  (for _array_element _outactors
    (bind _asbp_door_2button (cast `/Game/Blueprints/BP_Door_2Button` _array_element))
    (`/Game/Blueprints/BP_Door_2Button.CloseDoor` _asbp_door_2button)))

(fn `PlaySound`
  (`AudioComponent.Play` (`self.SC_ButtonClick`) 0.0))

(fn `UserConstructionScript`
  (set `self.ButtonValue` (`self.ButtonValue`)))