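; BP_WallButton is a wall button Blueprint whose press logic is present but disconnected, so it never runs.
; BeginPlay, the construction script and the ButtonAction event are empty, despite a comment about saving the origin location.
; The orphaned nodes gate presses on a "Pickup" component tag and DoOnce, briefly simulate physics, constrain to the XY plane, then call ButtonAction.
; A separate depress chain restores the origin location and clears IsPressed.
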(event `self.ReceiveBeginPlay`
  ; Save origin location
)

(event `ButtonAction`)

(fn `UserConstructionScript`)