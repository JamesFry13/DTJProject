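; A prank floor button that launches itself into the air when pressed with a pickup object.
; On BeginPlay it stores the button's world location as the effect origin.
; The first overlap by a component tagged Pickup marks it pressed, enables physics on the button, spawns a particle burst and fires upward and radial impulses, only once.
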(event `self.ReceiveBeginPlay`
  ; Save origin location
  (set `self.OriginLoc` (`SceneComponent.K2_GetComponentLocation` (`self.Button`))))

(event `self.OverlapCollider.OnComponentBeginOverlap`
  (params (OverlappedComponent :type "PrimitiveComponent Object Reference") (OtherActor :type "Actor Object Reference") (OtherComp :type "PrimitiveComponent Object Reference") (OtherBodyIndex :type Integer) (bFromSweep :type Boolean) (SweepResult :type "HitResult Structure (by ref)"))
  (bind _button (`self.Button`))
  ; Press
  (if (`ActorComponent.ComponentHasTag` OtherComp "Pickup")
    (`/Engine/EditorBlueprintResources/StandardMacros.DoOnce` false
      (:`Completed`
        (set `self.IsPressed?` true)
        (`PrimitiveComponent.SetSimulatePhysics` (`self.Button`) true)
        (`NiagaraFunctionLibrary.SpawnSystemAtLocation` "/Niagara/DefaultAssets/Templates/Systems/DirectionalBurst.DirectionalBurst" (`self.OriginLoc`))
        (`PrimitiveComponent.AddImpulse` _button (100.0 100.0 10000.0) "None" false)
        (`PhysicsObjectBlueprintLibrary.ApplyRadialImpulse` _button (`self.OriginLoc`) 100.0 10000.0 "RIF_Linear" true 0.0 false 1.0 100.0)))))

(fn `UserConstructionScript`)