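; BP_WallButtonNEW is an interactable wall button that opens and closes the BP_DoorBase doors whose DoorValue matches its ButtonValue.
; Interact toggles between press and release through IsPressed and a DoOnce, with a timeline sliding the red top in and out.
; Each press or release plays a click and searches all doors for matches.
; Opening sets a timer that closes them and raises the button, without clearing IsPressed.
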(event `self.ReceiveBeginPlay`
  ; Save origin location
)

(event `/Game/Blueprints/BPI_Interact.Interact`
  ; Press
  (if (`self.IsPressed?`)
    (`self.ButtonUpAnim`)
    ; Depress
    (set `self.IsPressed?` false)
    (`KismetSystemLibrary.Delay` 0.2)
    (`self.ButtonDepressed2`)
    (goto _label :!via `Reset`)
    (else
      (`self.ButtonDownAnim`)
      (`/Engine/EditorBlueprintResources/StandardMacros.DoOnce` false :!label _label
        (:`Completed`
          (set `self.IsPressed?` true)
          (`self.ButtonPressed2`))))))

(event `ButtonPressed2`
  ; Finds corresponding door by value
  (`AudioComponent.Play` (`self.SC_ButtonClick`) 0.0)
  (bind _outactors (`GameplayStatics.GetAllActorsOfClass` "/Game/Blueprints/BP_DoorBase.BP_DoorBase_C"))
  (for _array_element _outactors
    (bind _asbp_door_base (cast `/Game/Blueprints/BP_DoorBase` _array_element))
    (if (== (`self.ButtonValue`) (`/Game/Blueprints/BP_DoorBase.DoorValue` _asbp_door_base))
      (`/Game/Blueprints/BP_DoorBase.DoorOpen` _asbp_door_base)
      (`KismetSystemLibrary.K2_SetTimerDelegate` (delegate `ButtonDepressed2`) 3.5))))

(event `ButtonDepressed2`
  ; Comment
  (`AudioComponent.Play` (`self.SC_ButtonClick`) 0.0)
  (bind _outactors (`GameplayStatics.GetAllActorsOfClass` "/Game/Blueprints/BP_DoorBase.BP_DoorBase_C"))
  (for _array_element _outactors
    (bind _asbp_door_base (cast `/Game/Blueprints/BP_DoorBase` _array_element))
    (if (== (`self.ButtonValue`) (`/Game/Blueprints/BP_DoorBase.DoorValue` _asbp_door_base))
      (`/Game/Blueprints/BP_DoorBase.DoorClose` _asbp_door_base)
      (`self.ButtonUpAnim`))))

(event `ButtonDownAnim`
  (bind (_direction _newtrack_0) (`Timeline|ButtonDown` :!label _label_2)
    (:`Update`
      (`SceneComponent.K2_SetRelativeLocation` (`self.buttonredtop-1`) (`KismetMathLibrary.MakeVector` 0.0 0.0 (`KismetMathLibrary.Lerp` 0.0 -12.0 _newtrack_0)) false false))))

(event `ButtonUpAnim`
  (goto _label_2 :!via `Reverse`))

(fn `ButtonPressed`)

(fn `UserConstructionScript`
  (set `self.ButtonValue` (`self.ButtonValue`)))