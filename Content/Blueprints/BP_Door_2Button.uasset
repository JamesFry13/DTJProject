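; BP_Door_2Button is an unfinished door Blueprint, apparently meant to open with floor buttons.
; Its DoorOpen event gathers all BP_Floor_Button actors and loops over them with an empty body.
; A disconnected chain holds a DoOnce, a debug print and a timeline that would raise the Cube by lerping its relative Z.
; That chain's ButtonValue check compares the value to itself, and none of it runs.
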(event `self.DoorOpen`
  (bind _outactors (`GameplayStatics.GetAllActorsOfClass` "/Game/Blueprints/Buttons/BP_Floor_Button.BP_Floor_Button_C"))
  (for _array_element _outactors
    _))

(fn `UserConstructionScript`
  (`parent.UserConstructionScript`))