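; Door Blueprint, apparently a child of BP_DoorBase, that raises and lowers a panel with hydraulic effects.
; DoorOpen activates the SCHydraulicDoor component and plays a timeline that lerps Cube1's relative Z upward.
; DoorClose restarts that component after a brief delay and reverses the same timeline.
; The timeline's Finished output deactivates the component when movement ends in either direction.
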(event `self.DoorOpen`
  (`ActorComponent.SetActive` (`self.SC_HydraulicDoor`) true false)
  (bind (_direction _move) (`Timeline|Timeline_0` :!label _label)
    (:`Update`
      (`SceneComponent.K2_SetRelativeLocation` (`self.Cube1`) (`KismetMathLibrary.MakeVector` 0.0 0.0 (`KismetMathLibrary.Lerp` 130.0 800.0 _move)) false false))
    (:`Finished`
      (`ActorComponent.SetActive` (`self.SC_HydraulicDoor`) false false))))

(event `DoorClose`
  (`ActorComponent.SetActive` (`self.SC_HydraulicDoor`) false false)
  (`KismetSystemLibrary.Delay` 0.2)
  (`ActorComponent.SetActive` (`self.SC_HydraulicDoor`) true false)
  (goto _label :!via `Reverse`))

(fn `UserConstructionScript`
  (`parent.UserConstructionScript`))