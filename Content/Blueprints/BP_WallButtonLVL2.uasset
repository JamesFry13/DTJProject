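; BP_WallButtonLVL2 is a wall button whose Interact event opens the Brandon_3_Come_And_See level.
; It retains events that open or close every BP_DoorBase with a DoorValue matching its ButtonValue.
; A timeline played forward or in reverse slides the red button top down and up.
; The press-toggle logic linking animation to doors is disconnected, so Interact triggers neither.
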(event `self.ReceiveBeginPlay`
  ; Save origin location
)

(event `ButtonPressed2`
  ; Finds corresponding door by value
  (bind _outactors (`GameplayStatics.GetAllActorsOfClass` "/Game/Blueprints/BP_DoorBase.BP_DoorBase_C"))
  (for _array_element _outactors
    (bind _asbp_door_base (cast `/Game/Blueprints/BP_DoorBase` _array_element))
    (if (== (`self.ButtonValue`) (`/Game/Blueprints/BP_DoorBase.DoorValue` _asbp_door_base))
      (`/Game/Blueprints/BP_DoorBase.DoorOpen` _asbp_door_base))))

(event `ButtonDepressed2`
  ; Comment
  (bind _outactors (`GameplayStatics.GetAllActorsOfClass` "/Game/Blueprints/BP_DoorBase.BP_DoorBase_C"))
  (for _array_element _outactors
    (bind _asbp_door_base (cast `/Game/Blueprints/BP_DoorBase` _array_element))
    (if (== (`self.ButtonValue`) (`/Game/Blueprints/BP_DoorBase.DoorValue` _asbp_door_base))
      (`/Game/Blueprints/BP_DoorBase.DoorClose` _asbp_door_base))))

(event `ButtonDownAnim`
  (bind (_direction _newtrack_0) (`Timeline|ButtonDown` :!label _label)
    (:`Update`
      (`SceneComponent.K2_SetRelativeLocation` (`self.buttonredtop-1`) (`KismetMathLibrary.MakeVector` 0.0 0.0 (`KismetMathLibrary.Lerp` 0.0 -12.0 _newtrack_0)) false false))))

(event `ButtonUpAnim`
  (goto _label :!via `Reverse`))

(event `/Game/Blueprints/BPI_Interact.Interact`
  (`GameplayStatics.OpenLevelBySoftObjectPtr` "/Game/Levels/Brandon_3_Come_And_See.Brandon_3_Come_And_See"))

(fn `ButtonPressed`)

(fn `UserConstructionScript`
  (set `self.ButtonValue` (`self.ButtonValue`)))